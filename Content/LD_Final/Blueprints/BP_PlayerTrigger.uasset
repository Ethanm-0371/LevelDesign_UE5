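; BP_PlayerTrigger is a box trigger volume that detects when a player-class actor enters it.
; On begin overlap it compares the other actor's class to player pawn 0's class and, on a match, calls CharacterOn, an empty event here.
; The construction script applies the custom box size and outline color, and shows the box in game only when Debug is set.
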(event `self.Box.OnComponentBeginOverlap`
  (params (OverlappedComponent :type "PrimitiveComponent Object Reference") (OtherActor :type "Actor Object Reference") (OtherComp :type "PrimitiveComponent Object Reference") (OtherBodyIndex :type Integer) (bFromSweep :type Boolean) (SweepResult :type "HitResult Structure (by ref)"))
  (if (== (`GameplayStatics.GetObjectClass` OtherActor) (`GameplayStatics.GetObjectClass` (`GameplayStatics.GetPlayerPawn` 0)))
    (`self.Character On`)))

(event `Character On`)

(fn `UserConstructionScript`
  (bind _box (`self.Box`))
  ;[0.4948 0.3978 0.009404 0.5] Variables
  (`BoxComponent.SetBoxExtent` _box (`self.CustomSize`) true)
  (set `ShapeComponent.ShapeColor` (`self.OutlineColor`) _box)
  ;[0.5677 0.07392 0.07392 0.5] Debug
  (`SceneComponent.SetHiddenInGame` _box (not (`self.Debug`)) false))