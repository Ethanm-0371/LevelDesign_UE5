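; Collectible pickup actor that spins and bobs in the level, and destroys itself when its Characteron event fires.
; Each Tick rotates the static mesh in pitch by a fixed step, not scaled by delta time, and calls Play on a timeline.
; The timeline's UpDownMovement track drives a Lerp that sets the mesh's relative Z for the vertical movement.
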(event `self.Character On`
  (`self.K2_DestroyActor`))

(event `self.ReceiveTick`
  (params (DeltaSeconds :type "Float (single-precision)"))
  (`parent.ReceiveTick` DeltaSeconds)
  (`SceneComponent.K2_AddLocalRotation` (`self.StaticMesh`) (`KismetMathLibrary.MakeRotator` 0.0 1.0) false false)
  (bind (_direction _updownmovement) (`Timeline|Timeline`)
    (:`Update`
      (`SceneComponent.K2_SetRelativeLocation` (`self.StaticMesh`) (`KismetMathLibrary.MakeVector` 0.0 0.0 (`KismetMathLibrary.Lerp` -10.0 10.0 _updownmovement)) false false))))

(fn `UserConstructionScript`
  (`parent.UserConstructionScript`))